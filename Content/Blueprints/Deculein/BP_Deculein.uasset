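; BP_Deculein is a player-controlled pawn with a sprite that moves along the world X and Y axes.
; On BeginPlay it adds the IMC_TopDown Enhanced Input mapping context to its player controller's local player subsystem.
; IA_Move feeds AddMovementInput on both axes and mirrors the sprite through its X scale to face the horizontal input direction, keeping the last facing when that input is zero.
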(event Input|EnhancedActionEvents|EnhancedInputActionIA_Move
  (params (ActionValue :type Vector%202D%20Structure) (ElapsedSeconds :type Float%20%28double-precision%29) (TriggeredSeconds :type Float%20%28double-precision%29) (InputAction :type Input%20Action%20Object%20Reference :default "/Game/Input/Actions/IA_Move.IA_Move"))
  (bind (_x _y) (Math|Vector2D|BreakVector2D ActionValue))
  (bind _sprite (Variables|Default|GetSprite))
  (Pawn|Input|AddMovementInput "1.000000,0.000000,0.000000" _x false)
  (Math|Float|CompareFloat _x 0.0
    (:>
      (Transformation|SetRelativeScale3D _sprite "1.000000,1.000000,1.000000"))
    (:==
      _)
    (:<
      (Transformation|SetRelativeScale3D _sprite "-1.000000,1.000000,1.000000")))
  (Pawn|Input|AddMovementInput "0.000000,1.000000,0.000000" _y false))

(event EventBeginPlay
  (bind _asplayer_controller (Utilities|Casting|CastToPlayerController (Pawn|GetController)))
  (Input|AddMappingContext (PlayerController|LocalPlayerSubsystems|GetEnhancedInputLocalPlayerSubsystem _asplayer_controller) "/Game/Input/IMC_TopDown.IMC_TopDown" 0 "(bIgnoreAllPressedKeysUntilRelease=True,bForceImmediately=False,bNotifyUserSettings=False)"))

(event Collision|EventActorBeginOverlap
  (params (OtherActor :type Actor%20Object%20Reference)))

(event EventTick
  (params (DeltaSeconds :type Float%20%28single-precision%29)))

(fn ConstructionScript)